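; BP_Vase is a vase actor that plays a coin sound at the mesh's location and destroys itself on overlap.
; The overlap sequence casts player character 0 to BP_Player, then to BP_Enemy, each with its own sound.
; Both casts test the player character instead of the overlapping actor, so any overlap can trigger the player branch.
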(event Collision|EventActorBeginOverlap
  (params (OtherActor :type Actor%20Object%20Reference))
  (if true
    (Utilities|FlowControl|Sequence
      (:then_0
        (Utilities|Casting|CastToBP_Player (Game|GetPlayerCharacter 0))
        (Audio|PlaySoundatLocation "/Game/Interface_And_Item_Sounds/WAV/Coins_12.Coins_12" (Transformation|GetWorldLocation (Variables|Default|GetVase)) "0, 0, 0" 1.0 1.0 0.0 0 0 0 0)
        (Actor|DestroyActor))
      (:then_1
        (Utilities|Casting|CastToBP_Enemy (Game|GetPlayerCharacter 0))
        (Audio|PlaySoundatLocation "/Game/Interface_And_Item_Sounds/WAV/Coins_13.Coins_13" (Transformation|GetWorldLocation (Variables|Default|GetVase)) "0, 0, 0" 1.0 1.0 0.0 0 0 0 0)
        (Actor|DestroyActor)))))

(fn ConstructionScript)